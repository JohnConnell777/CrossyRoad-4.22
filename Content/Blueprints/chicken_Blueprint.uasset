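; Player chicken character for a Crossy Road-style hopper, with grid movement, water death and an idle eagle penalty.
; Inputs hop it 100 units with a cooldown, moving the spring arm along; forward hops randomly request new floor rows from the game mode.
; Hitting water flags death, and Tick sinks it with particle effects; 10 seconds without input spawns an eagle and destroys the mesh.
; Two functions show and hide a restart widget.
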(event `self.ReceiveBeginPlay`
  (if (`self.isDEAD`)
    _
    (else
      _))
  (if (`self.isDrowning`)
    (bind _returnvalue (`|CreateWidget` "/Game/Blueprints/UserInterface.UserInterface_C" null null))
    (set `self.RestartWidget` _returnvalue)))

(event `self.ReceiveTick`
  (params (DeltaSeconds :type "Float (single-precision)"))
  (bind (_returnvalue_x _returnvalue_y _returnvalue_z) (`KismetMathLibrary.BreakVector` (`self.K2_GetActorLocation`)))
  (bind (_returnvalue_x_2 _returnvalue_y_2) (`KismetMathLibrary.BreakVector` (`SceneComponent.K2_GetComponentLocation` (`self.StaticMesh1`))))
  (bind (_returnvalue_x_3 _returnvalue_y_3) (`KismetMathLibrary.BreakVector` (`SceneComponent.K2_GetComponentLocation` (`self.CapsuleComponent`))))
  (bind (_returnvalue_x_4 _returnvalue_y_4) (`KismetMathLibrary.BreakVector` (`SceneComponent.K2_GetComponentLocation` (`self.StaticMesh1`))))
  (bind (_returnvalue_x_5 _returnvalue_y_5) (`KismetMathLibrary.BreakVector` (`SceneComponent.K2_GetComponentLocation` (`self.CapsuleComponent`))))
  (if (`self.isDEAD`)
    (`SceneComponent.K2_SetWorldLocation` (`self.CapsuleComponent`) (`KismetMathLibrary.MakeVector` _returnvalue_x_3 _returnvalue_y_3 -15.0) false true)
    (if (`self.isDrowning`)
      (`PrimitiveComponent.SetCollisionResponseToAllChannels` (`self.CapsuleComponent`) "ECR_Overlap")
      (`SceneComponent.K2_SetWorldTransform` (`self.StaticMesh1`) (`KismetMathLibrary.MakeTransform` (`KismetMathLibrary.MakeVector` _returnvalue_x_2 _returnvalue_y_2 -40.0)) false false)
      (`/Engine/EditorBlueprintResources/StandardMacros.DoOnce` false
        (:`Completed`
          (`GameplayStatics.SpawnEmitterAtLocation` "/Game/Blueprints/WaterSplash.WaterSplash" (`KismetMathLibrary.MakeVector` _returnvalue_x_2 _returnvalue_y_2 20.0))
          (if (`self.isDEAD`)
            (`SceneComponent.K2_SetWorldLocation` (`self.CapsuleComponent`) (`KismetMathLibrary.MakeVector` _returnvalue_x_5 _returnvalue_y_5 -15.0) false true)
            (if (`self.isDEAD`)
              (`PrimitiveComponent.SetCollisionResponseToAllChannels` (`self.CapsuleComponent`) "ECR_Overlap")
              (`SceneComponent.K2_SetWorldTransform` (`self.StaticMesh1`) (`KismetMathLibrary.MakeTransform` (`KismetMathLibrary.MakeVector` _returnvalue_x_4 _returnvalue_y_4 -40.0)) false false)
              (`/Engine/EditorBlueprintResources/StandardMacros.DoOnce` false
                (:`Completed`
                  (`GameplayStatics.SpawnEmitterAtLocation` "/Game/Blueprints/FeatherBoom.FeatherBoom" (`KismetMathLibrary.MakeVector` _returnvalue_x_4 _returnvalue_y_4 20.0))))
              (else
                (`PrimitiveComponent.SetCollisionResponseToAllChannels` (`self.CapsuleComponent`) "ECR_Overlap")
                (`SceneComponent.K2_SetWorldTransform` (`self.StaticMesh1`) (`KismetMathLibrary.MakeTransform` (`KismetMathLibrary.MakeVector` _returnvalue_x_4 _returnvalue_y_4 -40.0)) false false)))
            (else
              (`ActorComponent.Deactivate` (`self.ParticleSystem`))
              ;[1 1 1] Spawn Eagle
              (if (not (`self.spawneagle`)) :!label _label
                (bind _output_get (set `self.SpawnDelay` (+ (`self.SpawnDelay`) DeltaSeconds)))
                (if (>= _output_get 10.0)
                  (`|SpawnActorFromClass` "/Game/Blueprints/Eagle_Blueprint.Eagle_Blueprint_C" (`KismetMathLibrary.MakeTransform` (`KismetMathLibrary.MakeVector` (+ _returnvalue_x 400.0) _returnvalue_y (+ _returnvalue_z 10.0)) (struct :`Pitch` 180.0 :`Roll` 180.0)) "Undefined" "OverrideRootScale" null null)
                  (set `self.spawneagle` true)
                  (`KismetSystemLibrary.Delay` 0.8)
                  (`ActorComponent.K2_DestroyComponent` (`self.StaticMesh1`))))))))
      (else
        (`PrimitiveComponent.SetCollisionResponseToAllChannels` (`self.CapsuleComponent`) "ECR_Overlap")
        (`SceneComponent.K2_SetWorldTransform` (`self.StaticMesh1`) (`KismetMathLibrary.MakeTransform` (`KismetMathLibrary.MakeVector` _returnvalue_x_2 _returnvalue_y_2 -40.0)) false false)))
    (else
      (`ActorComponent.Deactivate` (`self.ParticleSystem`))
      (goto _label))))

(event `self.StaticMesh1.OnComponentHit`
  (params (HitComponent :type "PrimitiveComponent Object Reference") (OtherActor :type "Actor Object Reference") (OtherComp :type "PrimitiveComponent Object Reference") (NormalImpulse :type "Vector Structure") (Hit :type "HitResult Structure (by ref)"))
  (if (`self.isDEAD`)
    (set `self.isDEAD` true)
    (else
      (cast `/Game/Blueprints/Water_BP` OtherActor)
      (set `self.isDEAD` true)
      (set `self.isDrowning` true))))

(event `InputAction|MoveBackard`
  (params (Key :type "Key Structure"))
  (bind _capsulecomponent (`self.CapsuleComponent`))
  (bind (_returnvalue_x _returnvalue_y _returnvalue_z) (`KismetMathLibrary.BreakVector` (`SceneComponent.K2_GetComponentLocation` (`self.SpringArm`))))
  (bind _returnvalue_x_2 (`KismetMathLibrary.BreakVector` (`SceneComponent.K2_GetComponentLocation` _capsulecomponent)))
  (:`Pressed`
    (set `self.SpawnDelay` 0.0)
    (if (not (`self.isJumping`))
      (`SceneComponent.K2_SetRelativeRotation` _capsulecomponent (struct :`Yaw` 180.0) false false)
      (`SceneComponent.K2_SetRelativeRotation` (`self.Mesh`) (struct :`Yaw` 180.0) false false)
      (set `self.isJumping` true)
      (`self.Jump`)
      (`SceneComponent.K2_AddWorldOffset` _capsulecomponent (-100.0 0.0 0.0) false false)
      (`SceneComponent.K2_SetWorldLocationAndRotation` (`self.SpringArm`) (`KismetMathLibrary.MakeVector` _returnvalue_x_2 _returnvalue_y _returnvalue_z) (`SceneComponent.K2_GetComponentRotation` (`self.SpringArm`)) false false)
      (`KismetSystemLibrary.Delay` 0.2)
      (set `self.isJumping` false)))
  (:`Released`
    (`AudioComponent.SetSound` (`self.Audiochicken`) "/Game/Blueprints/Chickendeepcluckbasicjump.Chickendeepcluckbasicjump")
    (`GameplayStatics.SpawnSoundAttached` "/Game/Blueprints/Chickendeepcluckbasicjump.Chickendeepcluckbasicjump" (`self.StaticMesh1`) "None" (0.0 0.0 0.0) (struct) "KeepRelativeOffset" false 1.0 1.0 0.0 null null)))

(event `InputAction|MoveForward`
  (params (Key :type "Key Structure"))
  (bind _capsulecomponent (`self.CapsuleComponent`))
  (bind _gamemode (`self.gamemode`))
  (bind (_returnvalue_x _returnvalue_y _returnvalue_z) (`KismetMathLibrary.BreakVector` (`SceneComponent.K2_GetComponentLocation` (`self.SpringArm`))))
  (bind _returnvalue_x_2 (`KismetMathLibrary.BreakVector` (`SceneComponent.K2_GetComponentLocation` _capsulecomponent)))
  (:`Pressed`
    (set `self.SpawnDelay` 0.0)
    (if (not (`self.isJumping`))
      (`SceneComponent.K2_SetRelativeRotation` :`self` _capsulecomponent)
      (`SceneComponent.K2_SetRelativeRotation` :`self` (`self.Mesh`))
      (set `self.isJumping` true)
      (`self.Jump`)
      (`SceneComponent.K2_AddWorldOffset` _capsulecomponent (100.0 0.0 0.0) false false)
      (`SceneComponent.K2_SetWorldLocationAndRotation` (`self.SpringArm`) (`KismetMathLibrary.MakeVector` _returnvalue_x_2 _returnvalue_y _returnvalue_z) (`SceneComponent.K2_GetComponentRotation` (`self.SpringArm`)) true false)
      (switch `int` (`KismetMathLibrary.RandomIntegerInRange` 0 4)
        (:`Default`
          _)
        (:`0`
          (`/Game/Blueprints/gamemodeBPP.CreateGrassFloors` _gamemode 1))
        (:`1`
          (`/Game/Blueprints/gamemodeBPP.CreateRoadFloors` _gamemode 1))
        (:`2`
          (`/Game/Blueprints/gamemodeBPP.CreateTrainTracksFloors` _gamemode 1))
        (:`3`
          (`/Game/Blueprints/gamemodeBPP.CreateWaterFloors` _gamemode 1)))
      (`KismetSystemLibrary.Delay` 0.2)
      (set `self.isJumping` false)))
  (:`Released`
    (`AudioComponent.SetSound` (`self.Audiochicken`) "/Game/Blueprints/Chickendeepcluckbasicjump.Chickendeepcluckbasicjump")
    (`GameplayStatics.SpawnSoundAttached` "/Game/Blueprints/Chickendeepcluckbasicjump.Chickendeepcluckbasicjump" (`self.StaticMesh1`) "None" (0.0 0.0 0.0) (struct) "KeepRelativeOffset" false 1.0 1.0 0.0 null null)))

(event `InputAction|MoveRight`
  (params (Key :type "Key Structure"))
  (bind _capsulecomponent (`self.CapsuleComponent`))
  (bind (_returnvalue_x _returnvalue_y _returnvalue_z) (`KismetMathLibrary.BreakVector` (`SceneComponent.K2_GetComponentLocation` (`self.SpringArm`))))
  (bind (_returnvalue_x_2 _returnvalue_y_2) (`KismetMathLibrary.BreakVector` (`SceneComponent.K2_GetComponentLocation` _capsulecomponent)))
  (:`Pressed`
    (set `self.SpawnDelay` 0.0)
    (if (not (`self.isJumping`))
      (`SceneComponent.K2_SetRelativeRotation` _capsulecomponent (struct :`Yaw` -270.0) false false)
      (`SceneComponent.K2_SetRelativeRotation` (`self.Mesh`) (struct :`Yaw` -270.0) false false)
      (set `self.isJumping` true)
      (`self.Jump`)
      (`SceneComponent.K2_AddWorldOffset` _capsulecomponent (0.0 100.0 0.0) false false)
      (`SceneComponent.K2_SetWorldLocationAndRotation` (`self.SpringArm`) (`KismetMathLibrary.MakeVector` _returnvalue_x _returnvalue_y_2 _returnvalue_z) (`SceneComponent.K2_GetComponentRotation` (`self.SpringArm`)) false false)
      (`KismetSystemLibrary.Delay` 0.2)
      (set `self.isJumping` false)))
  (:`Released`
    (`AudioComponent.SetSound` (`self.Audiochicken`) "/Game/Blueprints/Chickendeepcluckbasicjump.Chickendeepcluckbasicjump")
    (`GameplayStatics.SpawnSoundAttached` "/Game/Blueprints/Chickendeepcluckbasicjump.Chickendeepcluckbasicjump" (`self.StaticMesh1`) "None" (0.0 0.0 0.0) (struct) "KeepRelativeOffset" false 1.0 1.0 0.0 null null)))

(event `InputAction|MoveLeft`
  (params (Key :type "Key Structure"))
  (bind _capsulecomponent (`self.CapsuleComponent`))
  (bind (_returnvalue_x _returnvalue_y) (`KismetMathLibrary.BreakVector` (`SceneComponent.K2_GetComponentLocation` _capsulecomponent)))
  (bind (_returnvalue_x_2 _returnvalue_y_2 _returnvalue_z) (`KismetMathLibrary.BreakVector` (`SceneComponent.K2_GetComponentLocation` (`self.SpringArm`))))
  (:`Pressed`
    (set `self.SpawnDelay` 0.0)
    (if (not (`self.isJumping`))
      (`SceneComponent.K2_SetRelativeRotation` _capsulecomponent (struct :`Yaw` 270.0) false false)
      (`SceneComponent.K2_SetRelativeRotation` (`self.Mesh`) (struct :`Yaw` 270.0) false false)
      (set `self.isJumping` true)
      (`self.Jump`)
      (`SceneComponent.K2_AddWorldOffset` _capsulecomponent (0.0 -100.0 0.0) false false)
      (`SceneComponent.K2_SetWorldLocationAndRotation` (`self.SpringArm`) (`KismetMathLibrary.MakeVector` _returnvalue_x_2 _returnvalue_y _returnvalue_z) (`SceneComponent.K2_GetComponentRotation` (`self.SpringArm`)) false false)
      (`KismetSystemLibrary.Delay` 0.2)
      (set `self.isJumping` false)))
  (:`Released`
    (`AudioComponent.SetSound` (`self.Audiochicken`) "/Game/Blueprints/Chickendeepcluckbasicjump.Chickendeepcluckbasicjump")
    (`GameplayStatics.SpawnSoundAttached` "/Game/Blueprints/Chickendeepcluckbasicjump.Chickendeepcluckbasicjump" (`self.StaticMesh1`) "None" (0.0 0.0 0.0) (struct) "KeepRelativeOffset" false 1.0 1.0 0.0 null null)))

(fn `Displayrestartbutton`
  (bind _returnvalue (`GameplayStatics.GetPlayerController` 0))
  (`UserWidget.AddToViewport` (`self.RestartWidget`) 0)
  (`WidgetBlueprintLibrary.SetInputMode_UIOnlyEx` _returnvalue null)
  (set `PlayerController.bShowMouseCursor` true _returnvalue))

(fn `RestartGame`
  (bind _returnvalue (`GameplayStatics.GetPlayerController` 0))
  (set `self.isDEAD` false)
  (`Widget.RemoveFromParent` (`self.RestartWidget`))
  (`WidgetBlueprintLibrary.SetInputMode_GameOnly` _returnvalue)
  (set `PlayerController.bShowMouseCursor` false _returnvalue))

(fn `UserConstructionScript`)