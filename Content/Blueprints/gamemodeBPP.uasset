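; Game mode for a chicken road-crossing game that builds the level, creates the UI and respawns players.
; On BeginPlay it links itself to the chicken and UI widget, then lays grass, road, water and train-track strips along X using a shared FloorX offset.
; Tick converts the chicken's X position into a times-traveled count.
; RespawnPlayer spawns a new chicken at a player start and possesses it, without updating the stored Chicken reference.
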(event `Respawn Player`
  (params (Player :type "Controller Object Reference"))
  (bind _returnvalue (`|SpawnActorFromClass` "/Game/Blueprints/chicken_Blueprint.chicken_Blueprint_C" (`KismetMathLibrary.MakeTransform` (`self.K2_GetActorLocation` (`self.K2_FindPlayerStart` Player))) "Undefined" "OverrideRootScale" null null))
  (`Controller.Possess` Player _returnvalue))

(event `self.ReceiveBeginPlay`
  (bind _aschicken_blueprint (cast `/Game/Blueprints/chicken_Blueprint` (`GameplayStatics.GetPlayerCharacter` 0)))
  (set `self.chicken` _aschicken_blueprint)
  (bind _returnvalue (`|CreateWidget` "/Game/Blueprints/UserInterface.UserInterface_C" null self))
  (`UserWidget.AddToViewport` _returnvalue 0)
  (set `/Game/Blueprints/chicken_Blueprint.gamemode` self _aschicken_blueprint)
  (`self.CreateGrassFloors` 2)
  (`self.CreateRoadFloors` 1)
  (`self.CreateWaterFloors` 2)
  (`self.CreateTrainTracksFloors` 2))

(event `self.ReceiveTick`
  (params (DeltaSeconds :type "Float (single-precision)"))
  (bind _chickdist (`self.CheckChickenDistance`))
  (set `self.GettimesTraveled` (/ (`KismetMathLibrary.FTrunc` _chickdist) 100)))

(fn `CheckChickenDistance`
  (returns (chickdist :type "Float (double-precision)"))
  (bind _chicken (`self.chicken`))
  (bind _returnvalue_x (`KismetMathLibrary.BreakVector` (`self.K2_GetActorLocation` _chicken)))
  (if (`KismetSystemLibrary.IsValid` _chicken)
    (return (`KismetMathLibrary.Conv_IntToDouble` (`KismetMathLibrary.FTrunc` _returnvalue_x)))))

(fn `CreateGrassFloors`
  (params (NumFloors :type Integer))
  (for _ (range (+ NumFloors 1))
    (`|SpawnActorFromClass` "/Game/Blueprints/Grass_BP.Grass_BP_C" (`KismetMathLibrary.MakeTransform` (`KismetMathLibrary.MakeVector` (`self.floorX`))) "Undefined" "OverrideRootScale" null null)
    (set `self.floorX` (+ (`self.floorX`) 200.0))))

(fn `CreateRoadFloors`
  (params (NumFloors :type Integer))
  (for _ (range (+ NumFloors 1))
    (`|SpawnActorFromClass` "/Game/Blueprints/Road_BP.Road_BP_C" (`KismetMathLibrary.MakeTransform` (`KismetMathLibrary.MakeVector` (`self.floorX`))) "Undefined" "OverrideRootScale" null null)
    (set `self.floorX` (+ (`self.floorX`) 200.0))))

(fn `CreateTrainTracksFloors`
  (params (NumFloors :type Integer))
  (for _ (range (+ NumFloors 1))
    (`|SpawnActorFromClass` "/Game/Blueprints/TrainTracks_BP.TrainTracks_BP_C" (`KismetMathLibrary.MakeTransform` (`KismetMathLibrary.MakeVector` (`self.floorX`))) "Undefined" "OverrideRootScale" null null)
    (set `self.floorX` (+ (`self.floorX`) 200.0))))

(fn `CreateWaterFloors`
  (params (NumFloors :type Integer))
  (for _ (range (+ NumFloors 1))
    (`|SpawnActorFromClass` "/Game/Blueprints/Water_BP.Water_BP_C" (`KismetMathLibrary.MakeTransform` (`KismetMathLibrary.MakeVector` (`self.floorX`))) "Undefined" "OverrideRootScale" null null)
    (set `self.floorX` (+ (`self.floorX`) 200.0))))

(fn `UserConstructionScript`)