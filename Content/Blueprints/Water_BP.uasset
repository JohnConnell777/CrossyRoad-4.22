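; Water hazard actor that drowns the chicken and spawns logs, apparently for a road-crossing style game.
; A hit on its static mesh casts the other actor to chicken_Blueprint and sets its dead and drowning flags.
; From BeginPlay, the SpawnLog timeline's Update drives a five-second Delay, spacing out Log_BP spawns while it plays.
; Each log spawns at the mesh's location, offset along negative Y.
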(event `self.ReceiveBeginPlay`
  (`Timeline|SpawnLog`
    (:`Update`
      (`KismetSystemLibrary.Delay` 5.0)
      (`self.CreateandSetLog`))))

(event `self.StaticMesh.OnComponentHit`
  (params (HitComponent :type "PrimitiveComponent Object Reference") (OtherActor :type "Actor Object Reference") (OtherComp :type "PrimitiveComponent Object Reference") (NormalImpulse :type "Vector Structure") (Hit :type "HitResult Structure (by ref)"))
  (bind _aschicken_blueprint (cast `/Game/Blueprints/chicken_Blueprint` OtherActor))
  (set `/Game/Blueprints/chicken_Blueprint.isDEAD` true _aschicken_blueprint)
  (set `/Game/Blueprints/chicken_Blueprint.isDrowning` true _aschicken_blueprint))

(fn `CreateandSetLog`
  (bind (_returnvalue_x _returnvalue_y _returnvalue_z) (`KismetMathLibrary.BreakVector` (`SceneComponent.K2_GetComponentLocation` (`self.StaticMesh`))))
  (`|SpawnActorFromClass` "/Game/Blueprints/Log_BP.Log_BP_C" (`KismetMathLibrary.MakeTransform` (`KismetMathLibrary.MakeVector` _returnvalue_x (+ _returnvalue_y -1500.0) _returnvalue_z)) "Undefined" "OverrideRootScale" null null))

(fn `UserConstructionScript`)