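; Grass_BP is a grass ground piece that can randomly place a single coin, tree or rock on itself.
; On BeginPlay it randomly picks Coin_BP, Tree_BP or Rock_BP, then spawns it only if CoinSpawnRand modulo a random integer equals zero.
; The spawn takes X and Z from the static mesh's world location and randomizes Y across a fixed range centered on world zero.
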(event `self.ReceiveBeginPlay`
  (bind (_returnvalue_x _returnvalue_y _returnvalue_z) (`KismetMathLibrary.BreakVector` (`SceneComponent.K2_GetComponentLocation` (`self.StaticMesh`))))
  (bind (_returnvalue_x_2 _returnvalue_y_2 _returnvalue_z_2) (`KismetMathLibrary.BreakVector` (`SceneComponent.K2_GetComponentLocation` (`self.StaticMesh`))))
  (bind (_returnvalue_x_3 _returnvalue_y_3 _returnvalue_z_3) (`KismetMathLibrary.BreakVector` (`SceneComponent.K2_GetComponentLocation` (`self.StaticMesh`))))
  (switch `int` (`KismetMathLibrary.RandomInteger` 3)
    (:`0`
      (if (== (mod (`self.Coin Spawn Rand#`) (`KismetMathLibrary.RandomInteger` 5)) 0)
        (`|SpawnActorFromClass` "/Game/Blueprints/Coin_BP.Coin_BP_C" (`KismetMathLibrary.MakeTransform` (`KismetMathLibrary.MakeVector` _returnvalue_x (`KismetMathLibrary.RandomFloatInRange` -900.0 900.0) _returnvalue_z)) "Undefined" "OverrideRootScale" null null)))
    (:`1`
      (if (== (mod (`self.Coin Spawn Rand#`) (`KismetMathLibrary.RandomInteger` 5)) 0)
        (`|SpawnActorFromClass` "/Game/Blueprints/Tree_BP.Tree_BP_C" (`KismetMathLibrary.MakeTransform` (`KismetMathLibrary.MakeVector` _returnvalue_x_2 (`KismetMathLibrary.RandomFloatInRange` -900.0 900.0) _returnvalue_z_2)) "Undefined" "OverrideRootScale" null null)))
    (:`2`
      (if (== (mod (`self.Coin Spawn Rand#`) (`KismetMathLibrary.RandomInteger` 5)) 0)
        (`|SpawnActorFromClass` "/Game/Blueprints/Rock_BP.Rock_BP_C" (`KismetMathLibrary.MakeTransform` (`KismetMathLibrary.MakeVector` _returnvalue_x_3 (`KismetMathLibrary.RandomFloatInRange` -900.0 900.0) _returnvalue_z_3)) "Undefined" "OverrideRootScale" null null)))))

(fn `UserConstructionScript`)